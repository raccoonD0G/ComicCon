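; BP_Cam is an actor that receives the NDI network stream named "WebcamCutout" and drives a Media Plate component, apparently to display a webcam cutout.
; On BeginPlay and whenever the NDI finder reports changed network sources, NDIInit opens the media plate and scans the available sources.
; A matching stream is stored as the webcam connection, the NDI receiver starts on and switches to it, and the plate plays.
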(event `self.ReceiveBeginPlay`
  (`self.NDIInit`))

(event `self.NDIFinder.OnNetworkSourcesChanged`
  (params (InComponent :type "NDIFinderComponent Object Reference"))
  (`self.NDIInit`))

(fn `NDIInit`
  (`MediaPlateComponent.Open` (`self.MediaPlateComponent`))
  (for _array_element (`NDIFinderComponent.GetNetworkSources` (`self.NDIFinder`))
    (if (`KismetStringLibrary.EqualEqual_StrStr` (`.StreamName` (break `NDIConnectionInformation` _array_element)) "WebcamCutout")
      (set `self.WebcamConnection` _array_element)
      (`NDIReceiverComponent.StartReceiver` (`self.NDIReceiver`) (`self.WebcamConnection`))
      (`NDIReceiverComponent.ChangeConnection` (`self.NDIReceiver`) (`self.WebcamConnection`))
      (`MediaPlateComponent.Play` (`self.MediaPlateComponent`)))))

(fn `UserConstructionScript`)
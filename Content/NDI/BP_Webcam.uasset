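; BP_Webcam is an actor that connects to an NDI network stream named WebcamCutout to receive a webcam feed.
; On BeginPlay it sets its NDI media source to NR_Webcam and calls NDIConnect.
; NDIConnect searches the NDI finder's network sources by stream name and starts the receiver on the first match.
; The search runs only once, with no retry if the stream is absent.
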(event `self.ReceiveBeginPlay`
  (set `self.NDIMediaSource` "/Game/NDI/NR_Webcam.NR_Webcam")
  (`self.NDIConnect`))

(fn `NDIConnect`
  (for _array_element (`NDIFinderComponent.GetNetworkSources` (`self.NDIFinder`))
    (if (`KismetStringLibrary.EqualEqual_StrStr` (`.StreamName` (break `NDIConnectionInformation` _array_element)) "WebcamCutout")
      (set `self.WebcamConnection` _array_element)
      (`NDIReceiverComponent.StartReceiver` (`self.NDIReceiver`) (`self.WebcamConnection`))
      (`NDIReceiverComponent.ChangeConnection` (`self.NDIReceiver`) (`self.WebcamConnection`))
      (return))))

(fn `UserConstructionScript`)